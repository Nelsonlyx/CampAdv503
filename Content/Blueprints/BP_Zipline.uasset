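; BP_Zipline is a two-way zipline with a cable strung between AttachStart and AttachEnd, set up in both the construction script and BeginPlay.
; Collision volumes at each end call EnableZiplineOnOverlap on begin overlap, passing that end as the ride start and the other as the destination.
; Leaving either volume disables ziplining with zeroed points; the ride movement is not handled in these graphs.
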(event `self.ReceiveBeginPlay`
  (`self.InitializeCable`))

(event `self.CollisionStart.OnComponentBeginOverlap`
  (params (OverlappedComponent :type "PrimitiveComponent Object Reference") (OtherActor :type "Actor Object Reference") (OtherComp :type "PrimitiveComponent Object Reference") (OtherBodyIndex :type Integer) (bFromSweep :type Boolean) (SweepResult :type "HitResult Structure (by ref)"))
  ;[1 1 1] Allows Zipline on Overlap with the start of Zipline
  (`self.EnableZiplineOnOverlap` true (`SceneComponent.K2_GetComponentLocation` (`self.ZiplineStart`)) (`SceneComponent.K2_GetComponentLocation` (`self.ZiplineEnd`))))

(event `self.CollisionStart.OnComponentEndOverlap`
  (params (OverlappedComponent :type "PrimitiveComponent Object Reference") (OtherActor :type "Actor Object Reference") (OtherComp :type "PrimitiveComponent Object Reference") (OtherBodyIndex :type Integer))
  ;[1 1 1] Allows Zipline on Overlap with the start of Zipline
  (`self.EnableZiplineOnOverlap` false))

(event `self.CollisionEnd.OnComponentBeginOverlap`
  (params (OverlappedComponent :type "PrimitiveComponent Object Reference") (OtherActor :type "Actor Object Reference") (OtherComp :type "PrimitiveComponent Object Reference") (OtherBodyIndex :type Integer) (bFromSweep :type Boolean) (SweepResult :type "HitResult Structure (by ref)"))
  ;[1 1 1] Option to allow Zipline at the end of Zipline
  (`self.EnableZiplineOnOverlap` true (`SceneComponent.K2_GetComponentLocation` (`self.ZiplineEnd`)) (`SceneComponent.K2_GetComponentLocation` (`self.ZiplineStart`))))

(event `self.CollisionEnd.OnComponentEndOverlap`
  (params (OverlappedComponent :type "PrimitiveComponent Object Reference") (OtherActor :type "Actor Object Reference") (OtherComp :type "PrimitiveComponent Object Reference") (OtherBodyIndex :type Integer))
  ;[1 1 1] Option to allow Zipline at the end of Zipline
  (`self.EnableZiplineOnOverlap` false))

(fn `UserConstructionScript`
  (`self.InitializeCable`))